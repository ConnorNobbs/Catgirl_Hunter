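; Player character for the main game loop, which starts with a sword ability component and takes damage on contact with enemies or their projectiles.
; Capsule hits go to PlayerHit, which kills the enemy or destroys the projectile, subtracts its damage from health and updates the HUD.
; A timed invincibility window then blocks further hits.
; Nodes for the other abilities are present but unconnected, and no death handling happens here.
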(event `self.ReceiveBeginPlay`
  (`AddComponent|NODE_AddBP_swordAbility-0`))

(event `self.CapsuleComponent.OnComponentHit`
  (params (HitComponent :type "PrimitiveComponent Object Reference") (OtherActor :type "Actor Object Reference") (OtherComp :type "PrimitiveComponent Object Reference") (NormalImpulse :type "Vector Structure") (Hit :type "HitResult Structure (by ref)"))
  (`self.PlayerHit` OtherActor))

(fn `getPlayerActors`)

(fn `PlayerHit`
  (params (otherActor :type "Object Object Reference"))
  (locals (damage :type Integer))
  (if (`self.playerCanBeDamaged`)
    (bind _asbp_base_enemy (cast `/Game/Enemies/BP_BaseEnemy` otherActor)
      (:`then`
        (set `local.damage` (`/Game/Enemies/BP_BaseEnemy.damage` _asbp_base_enemy))
        (`/Game/Enemies/BP_BaseEnemy.TakeDamage` _asbp_base_enemy (`/Game/Enemies/BP_BaseEnemy.Health` _asbp_base_enemy)))
      (:`CastFailed`
        (bind _asbp_base_enemy_projectile (cast `/Game/Enemies/BP_BaseEnemyProjectile` otherActor))
        (set `local.damage` (`/Game/Enemies/BP_BaseEnemyProjectile.damage` _asbp_base_enemy_projectile))
        (`/Game/Enemies/BP_BaseEnemyProjectile.DestroyEnemyProjectile` _asbp_base_enemy_projectile)))
    (bind _output_get (set `self.currentHealth` (- (`self.currentHealth`) (`local.damage`))))
    (bind _asbp_my_hud (cast `/Game/UI/BP_MyHUD` (`PlayerController.GetHUD` (`GameplayStatics.GetPlayerController` 0))))
    (`/Game/UI/WB_MainGameLoopUI.OnPlayerCharacterDamaged` (`/Game/UI/BP_MyHUD.mainGameLoopUI` _asbp_my_hud) _output_get)
    (set `self.playerCanBeDamaged` false)
    (`KismetSystemLibrary.K2_SetTimer` null "setPlayerCanBeDamagedAgain" (`self.iFramesDuration`))))

(fn `setPlayerCanBeDamagedAgain`
  (set `self.playerCanBeDamaged` true))

(fn `UserConstructionScript`)