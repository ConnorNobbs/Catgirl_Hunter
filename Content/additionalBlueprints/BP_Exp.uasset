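; BP_Exp is an experience pickup that grants its value to the main game loop player character and destroys itself when its sphere overlaps them.
; Each Tick it compares its distance to the player against that character's pickup range and latches an attracted flag once inside.
; Once attracted, it homes toward the player with swept offsets, using a fixed step per frame without delta-time scaling.
; The construction script sets a fixed rotation.
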(event `self.Sphere.OnComponentBeginOverlap`
  (params (OverlappedComponent :type "PrimitiveComponent Object Reference") (OtherActor :type "Actor Object Reference") (OtherComp :type "PrimitiveComponent Object Reference") (OtherBodyIndex :type Integer) (bFromSweep :type Boolean) (SweepResult :type "HitResult Structure (by ref)"))
  (bind _asbp_main_game_loop_player_character (cast `/Game/PlayerCharacter/BP_MainGameLoopPlayerCharacter` OtherActor))
  (`/Game/PlayerCharacter/BP_MainGameLoopPlayerCharacter.addExp` _asbp_main_game_loop_player_character (`self.expvalue`))
  (`self.K2_DestroyActor`))

(event `self.ReceiveTick`
  (params (DeltaSeconds :type "Float (single-precision)"))
  (bind _returnvalue (`GameplayStatics.GetPlayerPawn` 0))
  (if (`self.beenattracted`)
    (`self.K2_AddActorWorldOffset` (* (`KismetMathLibrary.GetDirectionUnitVector` (`self.K2_GetActorLocation`) (`self.K2_GetActorLocation` (`GameplayStatics.GetPlayerPawn` 0))) (`self.movementspeed`)) true)
    (else
      (bind _asbp_main_game_loop_player_character (cast `/Game/PlayerCharacter/BP_MainGameLoopPlayerCharacter` _returnvalue))
      (if (< (`KismetMathLibrary.Vector_Distance` (`self.K2_GetActorLocation` _returnvalue) (`self.K2_GetActorLocation`)) (`/Game/PlayerCharacter/BP_MainGameLoopPlayerCharacter.exppickuprange` _asbp_main_game_loop_player_character))
        (set `self.beenattracted` true)))))

(fn `UserConstructionScript`
  (`self.K2_SetActorRotation` (struct :`Yaw` 90.0)))